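; Yellow environment block Blueprint that sets its color on BeginPlay and deals damage when the player controller actor leaves its Box1 trigger while the block is intact.
; Overlap events track the player and overlap state.
; A color and action-state check would destroy the block with sound and force feedback, but that chain is disconnected and Tick is empty, so it never runs.
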(event OnComponentBeginOverlap(Box1)
  (params (OverlappedComponent :type Primitive%20Component%20Object%20Reference) (OtherActor :type Actor%20Object%20Reference) (OtherComp :type Primitive%20Component%20Object%20Reference) (OtherBodyIndex :type Integer) (bFromSweep :type Boolean) (SweepResult :type Hit%20Result%20Structure%20%28by%20ref%29))
  (bind _asbp_dude (Utilities|Casting|CastToBP_RPPController OtherActor))
  (Variables|Default|SetbIsOverlapping true)
  (Variables|Default|SetPlayer _asbp_dude))

(event OnComponentEndOverlap(Box1)
  (params (OverlappedComponent :type Primitive%20Component%20Object%20Reference) (OtherActor :type Actor%20Object%20Reference) (OtherComp :type Primitive%20Component%20Object%20Reference) (OtherBodyIndex :type Integer))
  (bind _asbp_dude (Utilities|Casting|CastToBP_RPPController OtherActor))
  (if (not (Variables|Default|GetbIsDestoryed))
    (Development|PrintString "Hurt")
    (Default|DamageSyatem _asbp_dude 0.1)
    (Variables|Default|SetbIsOverlapping false)))

(event EventTick
  (params (DeltaSeconds :type Float%20%28single-precision%29)))

(event EventBeginPlay
  (Variables|Default|SetMyColor "NewEnumerator0"))

(fn ConstructionScript)